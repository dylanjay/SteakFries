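; Grid movement input component that turns player directional input into actions for the owner's BP_ActionScriptGenerator.
; On IA_Movement start it spawns a directional move actor, favoring X over Y, and submits it through TryAddAction.
; The MoveRight branch only spawns its actor and never submits it.
; IA_CancelAction resets the generator.
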(event `self.ReceiveBeginPlay`
  (set `self.Action Script Generator` (`Actor.GetComponentByClass` (`self.GetOwner`) "/Game/Blueprints/BP_ActionScriptGenerator.BP_ActionScriptGenerator_C")))

(event `EnhancedInput|/Game/Blueprints/IA_Movement`
  (params (ActionValue :type "Vector2D Structure") (ElapsedSeconds :type "Float (double-precision)") (TriggeredSeconds :type "Float (double-precision)") (InputAction :type "InputAction Object Reference" :default "/Game/Blueprints/IA_Movement.IA_Movement"))
  (bind _returnvalue (`KismetMathLibrary.MakeTransform` (0.0 0.0 0.0)))
  (bind (_x _y) (`KismetMathLibrary.BreakVector2D` ActionValue))
  (:`Started`
    (if (!= _x 0.0)
      (if (< (`KismetMathLibrary.FTrunc` _x) 0)
        (bind _returnvalue_2 (`|SpawnActorFromClass` "/Game/Blueprints/Actions/MoveLeft.MoveLeft_C" _returnvalue "AlwaysSpawn" "MultiplyWithRoot" null null))
        (`ActionScriptGeneratorComponent.TryAddAction` (`self.Action Script Generator`) _returnvalue_2)
        (else
          (`|SpawnActorFromClass` "/Game/Blueprints/Actions/MoveRight.MoveRight_C" _returnvalue "AlwaysSpawn" "MultiplyWithRoot" null null)))
      (elif (> (`KismetMathLibrary.FTrunc` _y) 0)
        (bind _returnvalue_3 (`|SpawnActorFromClass` "/Game/Blueprints/Actions/MoveUp.MoveUp_C" _returnvalue "AlwaysSpawn" "MultiplyWithRoot" null null))
        (`ActionScriptGeneratorComponent.TryAddAction` (`self.Action Script Generator`) _returnvalue_3)
        (else
          (bind _returnvalue_4 (`|SpawnActorFromClass` "/Game/Blueprints/Actions/MoveDown.MoveDown_C" _returnvalue "AlwaysSpawn" "MultiplyWithRoot" null null))
          (`ActionScriptGeneratorComponent.TryAddAction` (`self.Action Script Generator`) _returnvalue_4))))))

(event `EnhancedInput|/Game/Blueprints/IA_CancelAction`
  (params (ActionValue :type Boolean) (ElapsedSeconds :type "Float (double-precision)") (TriggeredSeconds :type "Float (double-precision)") (InputAction :type "InputAction Object Reference" :default "/Game/Blueprints/IA_CancelAction.IA_CancelAction"))
  (:`Triggered`
    (`ActionScriptGeneratorComponent.Reset` (`self.Action Script Generator`))))