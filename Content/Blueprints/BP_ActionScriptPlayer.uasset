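; Component that plays an ordered script of actions on its owning Pawn, which it caches on BeginPlay.
; PlayScript resets the index and stored array, then plays actions sequentially, binding to each action's completion delegate before playing it.
; Each completion starts a timer using that action's delay before the next plays, while the last one fires OnScriptComplete immediately.
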(event `self.ReceiveBeginPlay`
  (bind _aspawn (cast `Pawn` (`self.GetOwner`)))
  (set `self.Pawn` _aspawn))

(event `self.PlayScript`
  (params (Script :type "Array of Action Object Reference (by ref)"))
  (`self.Reset`)
  (set `self.Script` Script)
  (`self.Play Next Action`))

(event `Play Next Action`
  (bind _output (`|GetArrayItem` (`self.Script`) (`self.ActionIndex`)))
  (if (`KismetArrayLibrary.Array_IsValidIndex` (`self.Script`) (`self.ActionIndex`))
    (add `Action.OnActionCompleteDelegate` _output (delegate `On Action Complete`))
    (`Action.Play` _output (`self.Pawn`))))

(event `On Action Complete`
  (if (== (`self.ActionIndex`) (`KismetArrayLibrary.Array_LastIndex` (`self.Script`)))
    (`self.OnScriptComplete`)
    (else
      (`KismetSystemLibrary.K2_SetTimerDelegate` (delegate `OnDelayEnd`) (`Action.GetDelay` (`|GetArrayItem` (`self.Script`) (`self.ActionIndex`))))
      (`/Engine/EditorBlueprintResources/StandardMacros.IncrementInt` (`self.ActionIndex`)))))

(event `OnDelayEnd`
  (`self.Play Next Action`))

(fn `Reset`
  (set `self.ActionIndex` 0)
  (`KismetArrayLibrary.Array_Clear` (`self.Script`)))