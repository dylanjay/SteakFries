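; BP_GridMovementInput is an input handler that feeds the BP_ActionScriptGenerator component found on its owner at BeginPlay.
; IA_CancelAction resets that generator.
; A disconnected branch would spawn a left, right, up or down move actor from a 2D axis value, prioritizing X, and pass it to TryAddAction.
; No event triggers that branch, so only cancel input currently works.
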(event `self.ReceiveBeginPlay`
  (set `self.Action Script Generator` (`Actor.GetComponentByClass` (`self.GetOwner`) "/Game/Blueprints/BP_ActionScriptGenerator.BP_ActionScriptGenerator_C")))

(event `EnhancedInput|/Game/Blueprints/Input/IA_CancelAction`
  (params (ActionValue :type Boolean) (ElapsedSeconds :type "Float (double-precision)") (TriggeredSeconds :type "Float (double-precision)") (InputAction :type "InputAction Object Reference" :default "/Game/Blueprints/Input/IA_CancelAction.IA_CancelAction"))
  (:`Triggered`
    (`ActionScriptGeneratorComponent.Reset` (`self.Action Script Generator`))))