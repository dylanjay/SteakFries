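; BP_PlayerMovement is a component that turns player movement input into movement attempts on its owner's GridMovement component.
; Initialize caches that GridMovement component and, if the owning pawn is controlled by BP_PlayerController, adds the default Enhanced Input mapping context.
; When IA_Movement starts, it sends a truncated integer step on one axis, with X taking priority over Y, so a single input never requests a diagonal move.
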(event `EnhancedInput|/Game/Blueprints/IA_Movement`
  (params (ActionValue :type "Vector2D Structure") (ElapsedSeconds :type "Float (double-precision)") (TriggeredSeconds :type "Float (double-precision)") (InputAction :type "InputAction Object Reference" :default "/Game/Blueprints/IA_Movement.IA_Movement"))
  (bind (_x _y) (`KismetMathLibrary.BreakVector2D` ActionValue))
  (bind _gridmovementcomp (`self.GridMovementComp`))
  (:`Started`
    (if (!= _x 0.0)
      (`GridMovement.TryMoveX` _gridmovementcomp (`KismetMathLibrary.FTrunc` _x))
      (else
        (`GridMovement.TryMoveY` _gridmovementcomp (`KismetMathLibrary.FTrunc` _y))))))

(fn `Initialize`
  (bind _returnvalue (`self.GetOwner`))
  (set `self.GridMovementComp` (`Actor.GetComponentByClass` _returnvalue "/Script/SteakFries.GridMovement"))
  (bind _aspawn (cast `Pawn` _returnvalue))
  (bind _asbp_player_controller (cast `/Game/Blueprints/BP_PlayerController` (`Pawn.GetController` _aspawn)))
  (`EnhancedInputSubsystemInterface.AddMappingContext` (pcsubsystem `EnhancedInputLocalPlayerSubsystem` _asbp_player_controller) "/Game/Blueprints/IMC_Default.IMC_Default" 0 (struct)))