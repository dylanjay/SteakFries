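; BP_Player_Action is a player-side Blueprint that turns input into a queued script of actions and plays it on confirm.
; Attack input spawns an AttackAction actor and offers it to the owner's ActionScriptGenerator component.
; Confirm input passes the generated script to the owner's ActionScript component for playback.
; When playback completes, a bound event resets the generator.
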(event `self.ReceiveBeginPlay`
  (bind _returnvalue (`self.GetOwner`))
  (bind _output_get (set `self.Action Script` (`Actor.GetComponentByClass` _returnvalue "/Script/SteakFries.ActionScriptComponent")))
  (add `ActionScriptComponent.OnScriptComplete` _output_get (delegate `On Script Complete`))
  (set `self.Action Script Generator` (`Actor.GetComponentByClass` _returnvalue "/Script/SteakFries.ActionScriptGeneratorComponent")))

(event `On Script Complete`
  (`ActionScriptGeneratorComponent.Reset` (`self.Action Script Generator`)))

(event `EnhancedInput|/Game/Blueprints/IA_PlayerAttack`
  (params (ActionValue :type Boolean) (ElapsedSeconds :type "Float (double-precision)") (TriggeredSeconds :type "Float (double-precision)") (InputAction :type "InputAction Object Reference" :default "/Game/Blueprints/IA_PlayerAttack.IA_PlayerAttack"))
  (:`Started`
    (bind _returnvalue (`|SpawnActorFromClass` "/Game/Blueprints/Actions/AttackAction.AttackAction_C" (`KismetMathLibrary.MakeTransform` (0.0 0.0 0.0)) "AlwaysSpawn" "MultiplyWithRoot" null null))
    (`ActionScriptGeneratorComponent.TryAddAction` (`self.Action Script Generator`) _returnvalue)))

(event `EnhancedInput|/Game/Blueprints/IA_ConfirmAction`
  (params (ActionValue :type Boolean) (ElapsedSeconds :type "Float (double-precision)") (TriggeredSeconds :type "Float (double-precision)") (InputAction :type "InputAction Object Reference" :default "/Game/Blueprints/IA_ConfirmAction.IA_ConfirmAction"))
  (:`Started`
    (`ActionScriptComponent.PlayScript` (`self.Action Script`) (`ActionScriptGeneratorComponent.GetScript` (`self.Action Script Generator`)))))