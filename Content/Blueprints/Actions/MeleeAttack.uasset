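; MeleeAttack is a grid action that performs a pawn's sword strike on a neighbouring stage cell.
; Play jumps the pawn's PaperZD animation to its Attack node and binds to the player AnimBP's strike start and end events.
; Strike start spawns the sword attack actor one cell along the grid's second axis from the pawn.
; Strike end destroys that actor and signals action completion, if it is still valid.
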(event `self.Initialize`
  (params (InStageGrid :type "StageGrid Object Reference") (InCellLocation :type "StageCell Object Reference"))
  (bind _output_get (set `self.Stage Grid` InStageGrid))
  (`parent.Initialize` _output_get InCellLocation))

(event `self.Play`
  (params (Pawn :type "Pawn Object Reference"))
  (bind _animinstance (`PaperZDAnimationComponent.AnimInstance` (`Actor.GetComponentByClass` Pawn "/Script/PaperZD.PaperZDAnimationComponent")))
  (set `self.Pawn` Pawn)
  (`PaperZDAnimInstance.JumpToNode` _animinstance "Attack" "Main")
  (bind _asabp_player (cast `/Game/Blueprints/Animation/ABP_Player` _animinstance))
  (add `/Game/Blueprints/Animation/ABP_Player.StrikeStart` _asabp_player (delegate `On Strike Start`))
  (add `/Game/Blueprints/Animation/ABP_Player.StrikeEnd` _asabp_player (delegate `On Strike End`)))

(event `On Strike Start`
  (bind _stage_grid (`self.Stage Grid`))
  (bind _output_get (set `self.Attack Location` (`StageCell.BP_GetGridPoint` (`StageGrid.FindCharacter` _stage_grid (`self.Pawn`)))))
  (`/Engine/EditorBlueprintResources/StandardMacros.IncrementInt` (`|GetArrayItem` _output_get 1)
    (:`  `
      (`Actor.K2_AddActorLocalTransform` (`KismetMathLibrary.MakeTransform` (0.0 0.0 5.0)))
      (bind _returnvalue (`|SpawnActorFromClass` (`self.Sword Attack Class`) (`Actor.GetTransform` (`StageGrid.GetCell` _stage_grid (`self.Attack Location`))) "AlwaysSpawn" "MultiplyWithRoot" null (`self.Pawn`)))
      (set `self.Attack Actor` _returnvalue))))

(event `On Strike End`
  (bind _attack_actor (`self.Attack Actor`))
  (if (`KismetSystemLibrary.IsValid` _attack_actor)
    (`Actor.K2_DestroyActor` _attack_actor)
    (`self.OnActionCompleteDelegate`)))

(fn `UserConstructionScript`)