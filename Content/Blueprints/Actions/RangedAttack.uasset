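; Ranged attack action that makes a pawn fire a projectile on the stage grid.
; Play jumps the pawn's PaperZD animation to Attack and binds the ABP_Player strike-start event.
; On strike start, it spawns the projectile class at the cell one step along the grid's second axis from the pawn and shoots it along +X.
; The action-complete delegate call is unconnected, so the action never signals completion.
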(event `self.Initialize`
  (params (InCellLocation :type "StageCell Object Reference"))
  (set `self.Stage Grid` (`self.GetStageGrid`)))

(event `self.Play`
  (params (Pawn :type "Pawn Object Reference"))
  (bind _animinstance (`PaperZDAnimationComponent.AnimInstance` (`Actor.GetComponentByClass` Pawn "/Script/PaperZD.PaperZDAnimationComponent")))
  (set `self.Pawn` Pawn)
  (`PaperZDAnimInstance.JumpToNode` _animinstance "Attack" "Main")
  (bind _asabp_player (cast `/Game/Blueprints/Animation/ABP_Player` _animinstance))
  (add `/Game/Blueprints/Animation/ABP_Player.StrikeStart` _asabp_player (delegate `On Strike Start`)))

(event `On Strike Start`
  (bind _output_get (set `self.Attack Point` (`StageCell.BP_GetGridPoint` (`StageGrid.FindCharacter` (`self.Stage Grid`) (`self.Pawn`)))))
  (`/Engine/EditorBlueprintResources/StandardMacros.IncrementInt` (`|GetArrayItem` _output_get 1)
    (:`  `
      (`Actor.K2_AddActorLocalTransform` (`KismetMathLibrary.MakeTransform` (0.0 0.0 5.0)))
      (bind _returnvalue (`|SpawnActorFromClass` (`self.Projectile Attack Class`) (`Actor.GetTransform` (`StageGrid.GetCell` (`self.Stage Grid`) (`self.Attack Point`))) "AlwaysSpawn" "MultiplyWithRoot" null (`self.Pawn`)))
      (bind _output_get_2 (set `self.Attack Actor` _returnvalue))
      (bind _asbp_projectile_attack (cast `/Game/Blueprints/BP_ProjectileAttack` _output_get_2))
      (`/Game/Blueprints/BP_ProjectileAttack.ShootProjectile` _asbp_projectile_attack (1.0 0.0 0.0)))))

(fn `UserConstructionScript`)