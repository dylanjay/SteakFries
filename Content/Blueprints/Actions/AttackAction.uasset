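; AttackAction is a grid battle action that makes a pawn perform a sword attack on a neighboring cell.
; It jumps the pawn's PaperZD animation to the Attack node and binds to the player AnimInstance's strike start and end events.
; Strike start spawns the sword attack actor on the cell one step along the grid's second axis from the pawn.
; Strike end destroys that actor and signals action completion.
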(event `self.Initialize`
  (params (InStageGrid :type "StageGrid Object Reference") (InCellLocation :type "StageCell Object Reference"))
  (`parent.Initialize` InStageGrid InCellLocation)
  (bind _asbattle_game_mode (cast `BattleGameMode` (`GameplayStatics.GetGameMode`)))
  (set `self.Stage Grid` (`BattleGameMode.GetStageGrid` _asbattle_game_mode)))

(event `self.DoAction`
  (params (Pawn :type "Pawn Object Reference"))
  (bind _animinstance (`PaperZDAnimationComponent.AnimInstance` (`self.GetComponentByClass` Pawn "/Script/PaperZD.PaperZDAnimationComponent")))
  (set `self.Pawn` Pawn)
  (`PaperZDAnimInstance.JumpToNode` _animinstance "Attack" "Main")
  (bind _asabp_player (cast `/Game/Blueprints/ABP_Player` _animinstance))
  (add `/Game/Blueprints/ABP_Player.StrikeStart` _asabp_player (delegate `On Strike Start`))
  (add `/Game/Blueprints/ABP_Player.StrikeEnd` _asabp_player (delegate `On Strike End`)))

(event `On Strike Start`
  (bind _stage_grid (`self.Stage Grid`))
  (bind _returnvalue (`StageGrid.FindCharacter` _stage_grid (`self.Pawn`)))
  (bind _output_get (set `self.Attack Location` (`StageCell.GetGridLocation` _returnvalue)))
  (`/Engine/EditorBlueprintResources/StandardMacros.IncrementInt` (`|GetArrayItem` _output_get 1)
    (:`  `
      (bind _returnvalue_2 (`StageGrid.GetCell` _stage_grid (`self.Attack Location`)))
      (`self.K2_AddActorLocalTransform` (`KismetMathLibrary.MakeTransform` (0.0 0.0 5.0)))
      (bind _returnvalue_3 (`|SpawnActorFromClass` (`self.Sword Attack Class`) (`self.GetTransform` _returnvalue_2) "AlwaysSpawn" "MultiplyWithRoot" null (`self.Pawn`)))
      (set `self.Attack Actor` _returnvalue_3))))

(event `On Strike End`
  (bind _attack_actor (`self.Attack Actor`))
  (if (`KismetSystemLibrary.IsValid` _attack_actor)
    (`self.K2_DestroyActor` _attack_actor)
    (`self.OnActionCompleteDelegate`)))

(fn `UserConstructionScript`)