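; BP_PlayerMovementInput is a component on the StageGrid that previews the player's movement path across grid cells.
; It turns active while the player controller possesses a valid pawn and stores the cell under the cursor as the destination.
; HighlightPath requests a path from a given start to that destination and, on success, replaces the previously highlighted cells with the new path.
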(event `self.ReceiveBeginPlay`
  (bind _asplayer_controller_base (cast `PlayerControllerBase` (`GameplayStatics.GetPlayerController` 0)))
  (bind _output_get (set `self.PlayerController` _asplayer_controller_base))
  (add `Controller.OnPossessedPawnChanged` _output_get (delegate `OnPossessedPawnChanged`))
  (bind _asstage_grid (cast `StageGrid` (`self.GetOwner`)))
  (bind _output_get_2 (set `self.StageGrid` _asstage_grid))
  (add `StageGrid.OnBeginCursorOverCellDelegate` _output_get_2 (delegate `OnCursorOverCell`)))

(event `OnPossessedPawnChanged`
  (params (OldPawn :type "Pawn Object Reference") (NewPawn :type "Pawn Object Reference"))
  (set `self.Active` (`KismetSystemLibrary.IsValid` NewPawn)))

(event `OnCursorOverCell`
  (params (Cell :type "StageCell Object Reference"))
  (if (`self.Active`)
    (set `self.Destination` Cell)))

(fn `HighlightPath`
  (params (Start :type "StageCell Object Reference"))
  (if (and (`KismetSystemLibrary.IsValid` (`self.Destination`)) (`self.Active`))
    (bind (_outpath _returnvalue) (`StageGrid.TryFindPathToCell` (`self.StageGrid`) Start (`self.Destination`)))
    (if _returnvalue
      (`self.ResetPath`)
      (for _array_element _outpath
        (bind _asbp_stage_cell (cast `/Game/Blueprints/Stage/BP_StageCell` _array_element))
        (`/Game/Blueprints/Stage/BP_StageCell.SetHighlight` _asbp_stage_cell true)
        (`KismetArrayLibrary.Array_Add` (`self.HoveredPath`) _asbp_stage_cell)))))

(fn `ResetPath`
  (bind _hoveredpath (`self.HoveredPath`))
  (for _array_element _hoveredpath
    (`/Game/Blueprints/Stage/BP_StageCell.SetHighlight` _array_element false))
  (`KismetArrayLibrary.Array_Clear` _hoveredpath))