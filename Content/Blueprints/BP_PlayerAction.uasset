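; BP_PlayerAction is a component that handles the owning player pawn's input in a turn-based battle.
; The attack input spawns a RangedAttack and tries to queue it in the owner's ActionScriptGenerator; confirm passes that script to the ActionScriptPlayer and resets the generator.
; When playback completes, it resets the generator again and ends the turn through the BattleGameMode's TurnManager.
; A separate reset input reloads the current level.
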(event `self.ReceiveBeginPlay`
  (bind _aspawn (cast `Pawn` (`self.GetOwner`)))
  (set `self.Pawn` _aspawn)
  (bind _output_get (set `self.Action Script Player` (`Actor.GetComponentByClass` (`self.GetOwner`) "/Script/SteakFries.ActionScriptPlayerComponent")))
  (add `ActionScriptPlayerComponent.OnScriptComplete` _output_get (delegate `On Script Complete`))
  (set `self.Action Script Generator` (`Actor.GetComponentByClass` (`self.GetOwner`) "/Script/SteakFries.ActionScriptGeneratorComponent"))
  (bind _asbattle_game_mode (cast `BattleGameMode` (`GameplayStatics.GetGameMode`)))
  (set `self.TurnManager` (`BattleGameMode.GetTurnManager` _asbattle_game_mode)))

(event `On Script Complete`
  (`ActionScriptGeneratorComponent.Reset` (`self.Action Script Generator`))
  (`TurnManager.EndTurn` (`self.TurnManager`)))

(event `EnhancedInput|/Game/Blueprints/Input/IA_PlayerAttack`
  (params (ActionValue :type Boolean) (ElapsedSeconds :type "Float (double-precision)") (TriggeredSeconds :type "Float (double-precision)") (InputAction :type "InputAction Object Reference" :default "/Game/Blueprints/Input/IA_PlayerAttack.IA_PlayerAttack"))
  (:`Started`
    (bind _returnvalue (`|SpawnActorFromClass` "/Game/Blueprints/Actions/RangedAttack.RangedAttack_C" (`KismetMathLibrary.MakeTransform` (0.0 0.0 0.0)) "AlwaysSpawn" "MultiplyWithRoot" null null))
    (`ActionScriptGeneratorComponent.TryAddAction` (`self.Action Script Generator`) _returnvalue)))

(event `EnhancedInput|/Game/Blueprints/Input/IA_ConfirmAction`
  (params (ActionValue :type Boolean) (ElapsedSeconds :type "Float (double-precision)") (TriggeredSeconds :type "Float (double-precision)") (InputAction :type "InputAction Object Reference" :default "/Game/Blueprints/Input/IA_ConfirmAction.IA_ConfirmAction"))
  (:`Started`
    (`ActionScriptPlayerComponent.PlayScript` (`self.Action Script Player`) (`ActionScriptGeneratorComponent.GetScript` (`self.Action Script Generator`)))
    (`ActionScriptGeneratorComponent.Reset` (`self.Action Script Generator`))))

(event `EnhancedInput|/Game/Blueprints/Input/IA_Reset`
  (params (ActionValue :type Boolean) (ElapsedSeconds :type "Float (double-precision)") (TriggeredSeconds :type "Float (double-precision)") (InputAction :type "InputAction Object Reference" :default "/Game/Blueprints/Input/IA_Reset.IA_Reset"))
  (:`Started`
    (bind _returnvalue (`GameplayStatics.GetCurrentLevelName` true))
    (`GameplayStatics.OpenLevel` (`KismetStringLibrary.Conv_StringToName` _returnvalue))))